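; BP_Note is a rhythm-game note actor that travels along the NotePath spline of its RhythmTrack.
; MoveNote plays a Timeline from the start, with play rate set to the inverse of TimeToComplete.
; Each update maps the Timeline alpha to a distance along the spline and sets the actor's world location and rotation from that point.
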(event `self.ReceiveBeginPlay`)

(event `MoveNote`
  (`TimelineComponent.SetPlayRate` (`self.Timeline`) (/ 1.0 (`self.timeToComplete`)))
  (bind (_direction _newtrack_0) (`Timeline|Timeline` :!via `PlayFromStart`)
    (:`Update`
      (bind (_returnvalue_location _returnvalue_rotation) (`KismetMathLibrary.BreakTransform` (`SplineComponent.GetTransformAtDistanceAlongSpline` (`/Game/guitar_hero/BP_Track.NotePath` (`self.RhythmTrack`)) (`KismetMathLibrary.Lerp` 0.0 (`SplineComponent.GetSplineLength` (`/Game/guitar_hero/BP_Track.NotePath` (`self.RhythmTrack`))) _newtrack_0) "World" false)))
      (`self.K2_SetActorTransform` (`KismetMathLibrary.MakeTransform` _returnvalue_location _returnvalue_rotation)))))

(fn `UserConstructionScript`)