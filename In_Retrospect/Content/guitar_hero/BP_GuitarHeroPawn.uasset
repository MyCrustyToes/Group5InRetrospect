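; Player pawn for a five-lane Guitar Hero-style rhythm game, turning Enhanced Input note presses into score.
; Presses check BP_TrackManager's tracks; hits on lanes 2–5 destroy the note and fire a dispatcher that adds points and raises a multiplier clamped on Tick.
; Held inputs earn delta-time-scaled points on hold notes, otherwise setting a cooldown until release, while misses on lanes 2–5 lower the multiplier.
; Lane 1 only prints on hits, with its scoring disconnected.
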(event `self.ReceiveBeginPlay`
  (`EnhancedInputSubsystemInterface.AddMappingContext` (pcsubsystem `EnhancedInputLocalPlayerSubsystem` (`GameplayStatics.GetPlayerController` 0)) "/Game/guitar_hero/IA_GuitarHeroMappings.IA_GuitarHeroMappings" 0 (struct))
  (bind _returnvalue (`GameplayStatics.GetActorOfClass` "/Game/guitar_hero/BP_TrackManager.BP_TrackManager_C"))
  (bind _output_get (set `self.TrackManagerRef` _returnvalue))
  (set `self.noteScore` (`/Game/guitar_hero/BP_TrackManager.baseNoteScore` _output_get))
  (set `self.holdNoteScore` (`/Game/guitar_hero/BP_TrackManager.baseHoldNoteScore` _output_get))
  (add `self.OnNoteHitDispatcher` (delegate `OnNoteHitDispatcher_Event`)))

(event `OnNoteHitDispatcher_Event`
  (set `self.pointsTotal` (+ (`self.pointsTotal`) (* (`self.noteScore`) (`self.scoreMult`))))
  (set `self.scoreMult` (+ (`self.scoreMult`) 1)))

(event `self.ReceiveTick`
  (params (DeltaSeconds :type "Float (single-precision)"))
  (bind _scoremult (`self.scoreMult`))
  (if (< _scoremult 1)
    (set `self.scoreMult` 1)
    (elif (> _scoremult 3)
      (set `self.scoreMult` 3))))

(event `EnhancedInput|/Game/guitar_hero/IA_HitNote1`
  (params (ActionValue :type Boolean) (ElapsedSeconds :type "Float (double-precision)") (TriggeredSeconds :type "Float (double-precision)") (InputAction :type "InputAction Object Reference" :default "/Game/guitar_hero/IA_HitNote1.IA_HitNote1"))
  (bind _output (`|GetArrayItem` (`/Game/guitar_hero/BP_TrackManager.trackList` (`self.TrackManagerRef`))))
  (:`Triggered`
    (if (`/Game/guitar_hero/BP_Track.noteOnTarget` _output)
      (`KismetSystemLibrary.PrintString` "Hello")
      (else
        (if (`/Game/guitar_hero/BP_Track.holdNoteOnTarget` _output) :!label _label
          (if (not (`self.cooldownActive`)) :!label _label_2
            (set `self.pointsTotal` (+ (`self.pointsTotal`) (* (`self.holdNoteScore`) (`self.scoreMult`) (`GameplayStatics.GetWorldDeltaSeconds`)))))
          (else
            (set `self.cooldownActive` true :!label _label_3))))))
  (:`Ongoing`
    (goto _label))
  (:`Completed`
    (set `self.cooldownActive` false)))

(event `EnhancedInput|/Game/guitar_hero/IA_HitNote2`
  (params (ActionValue :type Boolean) (ElapsedSeconds :type "Float (double-precision)") (TriggeredSeconds :type "Float (double-precision)") (InputAction :type "InputAction Object Reference" :default "/Game/guitar_hero/IA_HitNote2.IA_HitNote2"))
  (bind _output (`|GetArrayItem` (`/Game/guitar_hero/BP_TrackManager.trackList` (`self.TrackManagerRef`)) 1))
  (:`Triggered`
    (if (`/Game/guitar_hero/BP_Track.noteOnTarget` _output)
      (`/Game/guitar_hero/BP_Track.destroyNote` _output true)
      (`self.OnNoteHitDispatcher`)
      (else
        (set `self.scoreMult` (- (`self.scoreMult`) 1) :!label _label_4)
        (`KismetSystemLibrary.PrintString` "fuck you"))))
  (:`Ongoing`
    (if (`/Game/guitar_hero/BP_Track.holdNoteOnTarget` _output)
      (goto _label_2)
      (else
        (goto _label_3))))
  (:`Completed`
    (set `self.cooldownActive` false)))

(event `EnhancedInput|/Game/guitar_hero/IA_HitNote3`
  (params (ActionValue :type Boolean) (ElapsedSeconds :type "Float (double-precision)") (TriggeredSeconds :type "Float (double-precision)") (InputAction :type "InputAction Object Reference" :default "/Game/guitar_hero/IA_HitNote3.IA_HitNote3"))
  (bind _output (`|GetArrayItem` (`/Game/guitar_hero/BP_TrackManager.trackList` (`self.TrackManagerRef`)) 2))
  (:`Triggered`
    (if (`/Game/guitar_hero/BP_Track.noteOnTarget` _output)
      (`/Game/guitar_hero/BP_Track.destroyNote` _output true)
      (`self.OnNoteHitDispatcher`)
      (else
        (goto _label_4))))
  (:`Ongoing`
    (if (`/Game/guitar_hero/BP_Track.holdNoteOnTarget` _output)
      (goto _label_2)
      (else
        (goto _label_3))))
  (:`Completed`
    (set `self.cooldownActive` false)))

(event `EnhancedInput|/Game/guitar_hero/IA_HitNote4`
  (params (ActionValue :type Boolean) (ElapsedSeconds :type "Float (double-precision)") (TriggeredSeconds :type "Float (double-precision)") (InputAction :type "InputAction Object Reference" :default "/Game/guitar_hero/IA_HitNote4.IA_HitNote4"))
  (bind _output (`|GetArrayItem` (`/Game/guitar_hero/BP_TrackManager.trackList` (`self.TrackManagerRef`)) 3))
  (:`Triggered`
    (if (`/Game/guitar_hero/BP_Track.noteOnTarget` _output)
      (`/Game/guitar_hero/BP_Track.destroyNote` _output true)
      (`self.OnNoteHitDispatcher`)
      (else
        (goto _label_4))))
  (:`Ongoing`
    (if (`/Game/guitar_hero/BP_Track.holdNoteOnTarget` _output)
      (goto _label_2)
      (else
        (goto _label_3))))
  (:`Completed`
    (set `self.cooldownActive` false)))

(event `EnhancedInput|/Game/guitar_hero/IA_HitNote5`
  (params (ActionValue :type Boolean) (ElapsedSeconds :type "Float (double-precision)") (TriggeredSeconds :type "Float (double-precision)") (InputAction :type "InputAction Object Reference" :default "/Game/guitar_hero/IA_HitNote5.IA_HitNote5"))
  (bind _output (`|GetArrayItem` (`/Game/guitar_hero/BP_TrackManager.trackList` (`self.TrackManagerRef`)) 4))
  (:`Triggered`
    (if (`/Game/guitar_hero/BP_Track.noteOnTarget` _output)
      (`/Game/guitar_hero/BP_Track.destroyNote` _output true)
      (`self.OnNoteHitDispatcher`)
      (else
        (goto _label_4))))
  (:`Ongoing`
    (if (`/Game/guitar_hero/BP_Track.holdNoteOnTarget` _output)
      (goto _label_2)
      (else
        (goto _label_3))))
  (:`Completed`
    (set `self.cooldownActive` false)))

(fn `UserConstructionScript`)