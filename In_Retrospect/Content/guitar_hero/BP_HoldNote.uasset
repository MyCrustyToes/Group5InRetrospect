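; Hold note actor for a Guitar Hero-style rhythm game that travels along a track's note path.
; It takes the track from its BP_Track owner on BeginPlay.
; Each tick it follows the NotePath spline at MoveSpeed, stretching its X scale relative to its own spline length.
; Once ReachedEnd is called, it moves along its forward vector while Duration counts down, then destroys itself.
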(event `self.ReceiveTick`
  (params (DeltaSeconds :type "Float (single-precision)"))
  (bind _returnvalue (* DeltaSeconds (`self.moveSpeed`)))
  (bind _output_get (set `self.distanceAlongTrack` (+ (`self.distanceAlongTrack`) _returnvalue)))
  (if (`self.HasReachedEnd`)
    (bind _output_get_2 (set `self.duration` (- (`self.duration`) DeltaSeconds)))
    (if (<= _output_get_2 0.0)
      (`self.K2_DestroyActor`)
      (else
        (`self.K2_AddActorWorldOffset` (* (`self.GetActorForwardVector`) (`KismetMathLibrary.MakeVector` _returnvalue _returnvalue _returnvalue)))))
    (elif (< _output_get (`SplineComponent.GetSplineLength` (`/Game/guitar_hero/BP_Track.NotePath` (`self.RhythmTrack`))))
      (bind (_returnvalue_location _returnvalue_rotation) (`KismetMathLibrary.BreakTransform` (`SplineComponent.GetTransformAtDistanceAlongSpline` (`/Game/guitar_hero/BP_Track.NotePath` (`self.RhythmTrack`)) _output_get "World" false)))
      (`self.K2_SetActorTransform` (`KismetMathLibrary.MakeTransform` _returnvalue_location _returnvalue_rotation (+ (`self.GetActorScale3D`) (`KismetMathLibrary.MakeVector` (/ _returnvalue (`SplineComponent.GetSplineLength` (`self.Spline`))))))))))

(event `self.ReceiveBeginPlay`
  (bind _asbp_track (cast `/Game/guitar_hero/BP_Track` (`self.GetOwner`)))
  (`/Engine/EditorBlueprintResources/StandardMacros.IsValid` _asbp_track
    (:`Is Valid`
      (set `self.RhythmTrack` _asbp_track))))

(event `ReachedEnd`
  (set `self.HasReachedEnd` true))

(fn `UserConstructionScript`)