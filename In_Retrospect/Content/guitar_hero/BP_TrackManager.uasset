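; Guitar-hero track manager that spawns notes on five string tracks from MetaSound cue labels.
; The construction script collects the BP_Track child actors.
; BeginPlay adds a watched audio component immediately and a second after the note's travel time to the collision point, so cues run ahead of the second.
; Each cue is parsed into note, fret and duration, then spawns a tap or hold note on the first matching track.
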(event `self.ReceiveBeginPlay`
  (bind _output (`|GetArrayItem` (`self.trackList`)))
  (bind (_returnvalue_x _returnvalue_y _returnvalue_z) (`KismetMathLibrary.BreakVector` (`SplineComponent.GetLocationAtSplinePoint` (`/Game/guitar_hero/BP_Track.NotePath` _output) 0 "World")))
  (bind (_returnvalue_x_2 _returnvalue_y_2) (`KismetMathLibrary.BreakVector` (`SceneComponent.K2_GetComponentLocation` (`/Game/guitar_hero/BP_Track.NoteCollision` _output))))
  (`|ExecutionSequence`
    (:`then_0`
      (`KismetSystemLibrary.Delay` (/ (`KismetMathLibrary.Vector_Distance` (`KismetMathLibrary.MakeVector` _returnvalue_x _returnvalue_y _returnvalue_z) (`KismetMathLibrary.MakeVector` _returnvalue_x_2 _returnvalue_y_2 _returnvalue_z)) (`.moveSpeed` (defaults `Object` (`self.noteClassRef`)))))
      (`AddComponent|NODE_AddAudioComponent-1`))
    (:`then_1`
      (bind _returnvalue (`AddComponent|NODE_AddAudioComponent-0`))
      (`MetaSoundOutputSubsystem.WatchOutput` (subsystem `MetaSoundOutputSubsystem`) _returnvalue "Cuelabel" (delegate `CueChange`) "None" "None"))))

(event `CueChange`
  (params (OutputName :type Name) (Output :type "MetaSoundOutput Structure (by ref)"))
  (bind (_success _returnvalue) (`MetasoundOutputBlueprintAccess.GetString` Output))
  (if (`KismetStringLibrary.NotEqual_StrStr` _returnvalue "none")
    (bind _returnvalue_2 (`KismetStringLibrary.FindSubstring` _returnvalue ","))
    (set `self.trackNote` (`KismetStringLibrary.GetSubstring` _returnvalue 0 _returnvalue_2))
    (bind _returnvalue_3 (+ _returnvalue_2 1))
    (set `self.fretPosition` (`KismetStringLibrary.Conv_StringToInt` (`KismetStringLibrary.GetSubstring` _returnvalue _returnvalue_3)))
    (set `self.noteDuration` (`KismetStringLibrary.Conv_StringToDouble` (`KismetStringLibrary.GetSubstring` _returnvalue (+ _returnvalue_3 2) (`KismetStringLibrary.Len` _returnvalue))))
    (for _array_element (`self.trackList`)
      (if (`KismetStringLibrary.EqualEqual_StrStr` (`|GetArrayItem` (`/Game/guitar_hero/BP_Track.noteList` _array_element) (- (`self.fretPosition`) 1)) (`self.trackNote`))
        (if (> (`self.noteDuration`) 0.0)
          (`/Game/guitar_hero/BP_Track.SpawnHoldNote` _array_element (`self.noteDuration`))
          (break)
          (else
            (`/Game/guitar_hero/BP_Track.SpawnNote` _array_element)
            (break)))))))

(fn `UserConstructionScript`
  (for _array_element (`|MakeArray` (`ChildActorComponent.ChildActor` (`self.String1`)) (`ChildActorComponent.ChildActor` (`self.String2`)) (`ChildActorComponent.ChildActor` (`self.String3`)) (`ChildActorComponent.ChildActor` (`self.String4`)) (`ChildActorComponent.ChildActor` (`self.String5`)))
    (bind _asbp_track (cast `/Game/guitar_hero/BP_Track` _array_element))
    (`/Engine/EditorBlueprintResources/StandardMacros.IsValid` _asbp_track
      (:`Is Valid`
        (`KismetArrayLibrary.Array_Add` (`self.trackList`) _asbp_track)))))