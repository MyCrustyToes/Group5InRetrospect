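; BP_LevelCamera is a level camera that follows the player along a spline, acting as a rail camera.
; On BeginPlay it becomes the first player controller's view target.
; Each tick it moves the SpringArm to the spline point closest to the player character.
; It also sets the arm's yaw from the spline's local-space direction there, with a fixed downward pitch and no roll.
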(event `self.ReceiveBeginPlay`
  (`PlayerController.SetViewTargetWithBlend` (`GameplayStatics.GetPlayerController` 0) self 0.0 "VTBlend_Linear" 0.0 false))

(event `self.ReceiveTick`
  (params (DeltaSeconds :type "Float (single-precision)"))
  (bind _springarm (`self.SpringArm`))
  (bind _returnvalue (`self.K2_GetActorLocation` (`GameplayStatics.GetPlayerCharacter` 0)))
  (bind (_returnvalue_roll _returnvalue_pitch _returnvalue_yaw) (`KismetMathLibrary.BreakRotator` (`KismetMathLibrary.Conv_VectorToRotator` (`SplineComponent.FindDirectionClosestToWorldLocation` (`self.Spline`) _returnvalue "Local"))))
  (`SceneComponent.K2_SetWorldLocation` _springarm (`SplineComponent.FindLocationClosestToWorldLocation` (`self.Spline`) _returnvalue "World") false false)
  (`SceneComponent.K2_SetWorldRotation` _springarm (`KismetMathLibrary.MakeRotator` 0.0 -30.0 _returnvalue_yaw) false false))

(fn `UserConstructionScript`)