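; BP_CrashCrab is a crab enemy that patrols between two points and hurts the player on contact.
; On BeginPlay it converts PointA and PointB from local to world space, then alternates AIMoveTo between them, flipping only on success.
; Any capsule overlap damages player 0, regardless of the overlapping actor.
; Any damage received triggers a delay, then starts the death animation and immediately destroys the crab.
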(event `self.ReceiveBeginPlay`
  (set `self.Point A` (`KismetMathLibrary.TransformLocation` (`self.GetTransform`) (`self.Point A`)))
  (set `self.Point B` (`KismetMathLibrary.TransformLocation` (`self.GetTransform`) (`self.Point B`)))
  (`self.MoveToPoint`))

(event `MoveToPoint`
  (bind (_returnvalue_x _returnvalue_y _returnvalue_z) (`KismetMathLibrary.BreakVector` (`KismetMathLibrary.SelectVector` (`self.Point B`) (`self.Point A`) (`self.A-B`))))
  (`|AIMoveTo` self (`KismetMathLibrary.MakeVector` _returnvalue_x _returnvalue_y _returnvalue_z) null
    (:`OnSuccess`
      (set `self.A-B` (not (`self.A-B`)))
      (`self.MoveToPoint`))))

(event `self.ReceiveAnyDamage`
  (params (Damage :type "Float (single-precision)") (DamageType :type "DamageType Object Reference") (InstigatedBy :type "Controller Object Reference") (DamageCauser :type "Actor Object Reference"))
  (`KismetSystemLibrary.Delay` 1.0)
  (`SkeletalMeshComponent.PlayAnimation` (`self.Mesh`) "/Game/Crash_Assets/CrashCrab/crab_death_Anim.crab_death_Anim" true)
  (`self.K2_DestroyActor`))

(event `self.CapsuleComponent.OnComponentBeginOverlap`
  (params (OverlappedComponent :type "PrimitiveComponent Object Reference") (OtherActor :type "Actor Object Reference") (OtherComp :type "PrimitiveComponent Object Reference") (OtherBodyIndex :type Integer) (bFromSweep :type Boolean) (SweepResult :type "HitResult Structure (by ref)"))
  (`GameplayStatics.ApplyDamage` (`GameplayStatics.GetPlayerCharacter` 0) 1.0 null null "/Script/Engine.DamageType"))

(fn `UserConstructionScript`)